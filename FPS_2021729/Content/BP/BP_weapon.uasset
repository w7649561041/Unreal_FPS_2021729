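; Weapon Blueprint with automatic fire and magazine-based ammo, built around the SKKA74UX mesh.
; Holding the shot input runs a Delay loop that spawns BP_bullet and a muzzle flash at the "slot" socket, using one loaded round every Duration.
; Firing stops on release or when Onload is empty.
; The reloading event tops Onload up to Clip from the Reload reserve, limited to what remains.
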(event `InputAction|shot`
  (params (Key :type "Key Structure"))
  (bind _sk_ka74u_x (`self.SK_KA74U_X`))
  ;[1 1 1] shot
  (:`Pressed`
    (set `self.shooting` true)
    (if (and (> (`self.onload`) 0) (`self.shooting`)) :!label _label
      (`|SpawnActorFromClass` "/Game/BP/BP_bullet.BP_bullet_C" (`SceneComponent.GetSocketTransform` (`self.SK_KA74U_X`) "slot" "RTS_World") "Undefined" "OverrideRootScale" null null)
      (`GameplayStatics.SpawnEmitterAtLocation` "/Game/InfinityBladeEffects/Effects/FX_Monsters/FX_Monster_Gruntling/Master/P_BackPack_MuzzleFlash.P_BackPack_MuzzleFlash" (`SceneComponent.GetSocketLocation` _sk_ka74u_x "slot") (`SceneComponent.GetSocketRotation` _sk_ka74u_x "None") (0.1 0.1 0.1))
      (set `self.onload` (- (`self.onload`) 1))
      (`KismetSystemLibrary.Delay` (`self.duration`))
      (goto _label)))
  (:`Released`
    (set `self.shooting` false)))

(event `reloading`
  ;[1 1 1] Reloading
  (set `self.difference` (- (`self.clip`) (`self.onload`)))
  (if (not (>= (`self.reload`) (`self.difference`)))
    (set `self.difference` (`self.reload`)))
  (set `self.onload` (+ (`self.onload`) (`self.difference`)))
  (set `self.reload` (- (`self.reload`) (`self.difference`))))

(fn `UserConstructionScript`)