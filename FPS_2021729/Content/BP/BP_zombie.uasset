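; Zombie enemy that wanders to random reachable points until it sees the player or survives a bullet hit, then chases and attacks.
; A looping AIMoveTo flow switches on a See flag; failed chases return to wandering with random pauses.
; Attacks halt movement and briefly enable HitBox overlaps to damage the player.
; Bullet overlaps reduce HP; death triggers ragdoll, increments the game mode's kill count and destroys the actor after a delay.
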(event `self.PawnSensing.OnSeePawn`
  (params (Pawn :type "Pawn Object Reference"))
  (bind _hitbox (`self.HitBox`))
  (bind _charactermovement (`self.CharacterMovement`))
  ;[1 1 1] GetPlayer
  (bind _asbp_ch (cast `/Game/BP/BP_ch` Pawn))
  (set `self.As BP Ch` _asbp_ch)
  (set `self.See` true :!label _label)
  (set `self.RandomTime` 0.0)
  (`/Engine/EditorBlueprintResources/StandardMacros.DoOnce` false
    (:`Completed`
      ;[1 1 1] SeeBool
      (if (`self.See`) :!label _label_2
        ;[1 1 1] SeePlayer
        (`|AIMoveTo` self (0.0 0.0 0.0) (`self.As BP Ch`)
          (:`OnSuccess`
            ;[1 1 1] attack
            (set `self.Attacking` true)
            (set `CharacterMovementComponent.MaxWalkSpeed` 0.0 _charactermovement)
            (`KismetSystemLibrary.Delay` 1.0)
            (set `PrimitiveComponent.bGenerateOverlapEvents` true _hitbox)
            (`KismetSystemLibrary.Delay` 0.5)
            (set `PrimitiveComponent.bGenerateOverlapEvents` false _hitbox)
            (`KismetSystemLibrary.Delay` 1.0)
            (set `CharacterMovementComponent.MaxWalkSpeed` 600.0 _charactermovement)
            (set `self.Attacking` false)
            (goto _label_2))
          (:`OnFail`
            (set `self.See` false)
            (set `self.RandomTime` 3.0)
            (goto _label_2)))
        (else
          ;[1 1 1] RandomMove
          (`|AIMoveTo` self (`NavigationSystemV1.K2_GetRandomReachablePointInRadius` (`SceneComponent.GetSocketLocation` (`self.CapsuleComponent`) "None") (`self.Radius`) null null) null
            (:`then`
              ;[1 1 1] RandomStop
              (`KismetSystemLibrary.Delay` (* (`KismetMathLibrary.RandomFloat`) (`self.RandomTime`)))
              (goto _label_2))))))))

(event `self.ReceiveBeginPlay`
  (`|ExecutionSequence`
    (:`then_0`
      (goto _label_2))
    (:`then_1`
      (bind _asbp_mode (cast `/Game/BP/BP_mode` (`GameplayStatics.GetGameMode`)))
      (set `self.As BP Mode` _asbp_mode))
    (:`then_2`
      ;[1 1 1] ignoreCol
      (`PrimitiveComponent.IgnoreComponentWhenMoving` (`self.CapsuleComponent`) (`self.HitBox`) false))))

(event `self.CapsuleComponent.OnComponentBeginOverlap`
  (params (OverlappedComponent :type "PrimitiveComponent Object Reference") (OtherActor :type "Actor Object Reference") (OtherComp :type "PrimitiveComponent Object Reference") (OtherBodyIndex :type Integer) (bFromSweep :type Boolean) (SweepResult :type "HitResult Structure (by ref)"))
  (bind _as_bp_mode (`self.As BP Mode`))
  ;[1 1 1] injured
  (cast `/Game/BP/BP_bullet` OtherActor)
  (bind _dead (`self.injured` 0.1))
  (if _dead
    (set `/Game/BP/BP_mode.殺死怪物數量` (+ (`/Game/BP/BP_mode.殺死怪物數量` _as_bp_mode) 1) _as_bp_mode)
    (`KismetSystemLibrary.Delay` 3.0)
    (`self.K2_DestroyActor`)
    (else
      (goto _label))))

(event `self.HitBox.OnComponentBeginOverlap`
  (params (OverlappedComponent :type "PrimitiveComponent Object Reference") (OtherActor :type "Actor Object Reference") (OtherComp :type "PrimitiveComponent Object Reference") (OtherBodyIndex :type Integer) (bFromSweep :type Boolean) (SweepResult :type "HitResult Structure (by ref)"))
  ;[1 1 1] zombie_ATK
  (bind _asbp_ch (cast `/Game/BP/BP_ch` OtherActor))
  (`/Game/BP/BP_ch.injured` _asbp_ch (`self.ATK_zombie`)))

(fn `injured`
  (params (injured :type "Float (double-precision)"))
  (returns (Dead :type Boolean))
  (bind _output_get (set `self.HP` (- (`self.HP`) injured)))
  (if (<= _output_get 0.0)
    (`PrimitiveComponent.SetSimulatePhysics` (`self.Mesh`) true)
    (`PrimitiveComponent.SetCollisionEnabled` (`self.CapsuleComponent`) "NoCollision")
    (return true)
    (else
      (return false))))

(fn `UserConstructionScript`)